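; BP_Laser is a laser actor that fires a beam along its forward vector up to a set distance.
; On BeginPlay it applies its color to the Niagara beam and impact effects.
; Each tick it line-traces on the Camera channel, with a one-frame debug draw, to set the beam's end at the hit or maximum range.
; The impact effect moves to the hit point and shows only when something blocks the beam.
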(event `self.ReceiveBeginPlay`
  (bind _returnvalue (`KismetMathLibrary.Conv_ColorToLinearColor` (`self.Color`)))
  (`FXSystemComponent.SetColorParameter` (`self.Niagara_Laser`) "Color" _returnvalue)
  (`FXSystemComponent.SetColorParameter` (`self.Niagara_LaserImpact`) "Color" _returnvalue))

(event `self.ReceiveTick`
  (params (DeltaSeconds :type "Float (single-precision)"))
  (bind _returnvalue (`self.K2_GetActorLocation`))
  (bind _niagara_laserimpact (`self.Niagara_LaserImpact`))
  (bind _output_get (set `self.TraceEnd` (+ _returnvalue (* (`self.GetActorForwardVector`) (`self.Distance`)))))
  (bind _outhit (`KismetSystemLibrary.LineTraceSingle` :`Start` _returnvalue :`End` _output_get :`TraceChannel` "TraceTypeQuery2" :`DrawDebugType` "ForOneFrame"))
  (bind _output_get_2 (set `self.Out Hit Blocking Hit` (`GameplayStatics.BreakHitResult` _outhit)))
  (bind _output_get_3 (set `self.Out Hit Location` (`.Location` (`GameplayStatics.BreakHitResult` _outhit))))
  (`FXSystemComponent.SetVectorParameter` (`self.Niagara_Laser`) "LaserEnd" (select `bool` _output_get_2 :`false` (`self.TraceEnd`) :`true` _output_get_3))
  (`SceneComponent.SetVisibility` _niagara_laserimpact (`self.Out Hit Blocking Hit`) false)
  (`SceneComponent.K2_SetWorldLocation` _niagara_laserimpact (`self.Out Hit Location`) false false))

(fn `UserConstructionScript`)